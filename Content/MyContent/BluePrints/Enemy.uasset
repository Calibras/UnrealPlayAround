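; Enemy that chases the player once it spots a pawn and deals damage on contact.
; PawnSensing sets a seen flag, never cleared here, and triggers an AI move toward the first player character.
; Hits from a first-person projectile destroy it outright.
; Hits on the player character subtract Damage from its Health and print the result, gated by a short delay-based attack cooldown.
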(event OnSeePawn(PawnSensing)
  (params (Pawn :type Pawn%20Object%20Reference))
  (Variables|Default|SetisPlayerSeen true)
  (CallFunction|FollowPlayer))

(event Custom|FollowPlayer
  (if (Variables|Default|GetisPlayerSeen)
    (AI|AIMoveTo self "0, 0, 0" (Game|GetPlayerCharacter 0) 5.0 false)))

(event EventBeginPlay)

(event Collision|EventActorBeginOverlap
  (params (OtherActor :type Actor%20Object%20Reference)))

(event EventTick
  (params (DeltaSeconds :type Float%20%28single-precision%29)))

(event Collision|EventHit
  (params (MyComp :type Primitive%20Component%20Object%20Reference) (Other :type Actor%20Object%20Reference) (OtherComp :type Primitive%20Component%20Object%20Reference) (bSelfMoved :type Boolean) (HitLocation :type Vector :default "0, 0, 0") (HitNormal :type Vector :default "0, 0, 0") (NormalImpulse :type Vector :default "0, 0, 0") (Hit :type Hit%20Result%20Structure%20%28by%20ref%29))
  (Utilities|Casting|CastToBP_FirstPersonProjectile Other
    (:then
      (Actor|DestroyActor))
    (:CastFailed
      ;[1 1 1] Not Projectile, its a player? deal damage
      (bind _asbp_first_person_character (Utilities|Casting|CastToBP_FirstPersonCharacter Other))
      (if (Variables|Default|GetattackReady)
        (Variables|Default|SetattackReady false)
        (bind _output_get (Variables|/Game/FirstPerson/Blueprints/BP_FirstPersonCharacter.BP_FirstPersonCharacter_C|Sethealth _asbp_first_person_character (- (Variables|/Game/FirstPerson/Blueprints/BP_FirstPersonCharacter.BP_FirstPersonCharacter_C|Gethealth _asbp_first_person_character) (Variables|Default|Getdamage))))
        (Development|PrintString (Utilities|String|ToString(Float) _output_get))
        (Utilities|FlowControl|Delay 1.0)
        (Variables|Default|SetattackReady true)))))

(fn ConstructionScript)